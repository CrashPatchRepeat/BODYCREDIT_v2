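; BP_CNoxController is a player controller that sets up the root UI and opening screen when it possesses a pawn.
; On possess, it creates WBP_MainMenu, adds it to the viewport and registers it with the game instance subsystem as the primary layout.
; It then pushes a tag-resolved soft widget: the main menu screen on the Frontend stack for StartMap, otherwise the HUD on the GameHud stack.
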(event EventBeginPlay)

(event EventTick
  (params (DeltaSeconds :type Float%20%28single-precision%29)))

(event EventPossess
  (params (PossessedPawn :type Pawn%20Object%20Reference))
  (bind _returnvalue (UserInterface|CreateWidget "/Game/UIs/Items/Common/WBP_MainMenu.WBP_MainMenu_C" self))
  (UserInterface|Viewport|AddtoViewport _returnvalue 0)
  (Class|CGameInstanceSubsystem|RegisterCreatedPrimaryLayoutWidget (Subsystems|GetCGameInstanceSubsystem) _returnvalue)
  (bind _returnvalue_2 (Game|GetCurrentLevelName true))
  (if (Utilities|Enum|Equal(Enum) _returnvalue_2 "StartMap")
    (|PushSoftWidget self (Class|CFunctionLibrary|GetSoftWidgetClassbyTag "(TagName=\"WidgetStack.Frontend.MainMenuScreen\")") "(TagName=\"WidgetStack.Frontend\")" true)
    (else
      (|PushSoftWidget self (Class|CFunctionLibrary|GetSoftWidgetClassbyTag "(TagName=\"WidgetStack.GameHud.Hud\")") "(TagName=\"WidgetStack.GameHud\")" true))))

(fn ConstructionScript)