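; Standing light prop from a sci-fi kit, with a tiltable head, optional second lamp, and on/off and flickering options.
; The construction script applies these to the meshes through a dynamic emissive material or an off material; light component calls are disconnected.
; StartExtract starts a looping timer that ping-pongs the material color between two colors.
; EndChangeColor stops the timer and sets a final color.
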(event Custom|ChangeTempColor
  (params (NewColor :type Linear%20Color%20Structure))
  (bind _mi_temporarylight (Variables|Default|GetMI_TemporaryLight))
  (Rendering|Material|SetVectorParameterValue _mi_temporarylight "Light_Color" NewColor :!class /Script/Engine.MaterialInstanceDynamic)
  (Rendering|Material|SetMaterial (Variables|Default|GetSM_StandingLight_A1_RotatingPart_N) 1 _mi_temporarylight)
  (Rendering|Material|SetMaterial (Variables|Default|GetSM_StandingLight_A1_RotatingPart_N1) 1 _mi_temporarylight)
  (Variables|Light|SetColor NewColor))

(event Custom|CalcLerpColor
  (Variables|Default|SetAlpha (Math|Float|Clamp(Float) (+ (Variables|Default|GetAlpha) (Utilities|Time|GetWorldDeltaSeconds))))
  (if (Variables|Default|GetColorMove)
    (CallFunction|ChangeTempColor (Math|Color|Lerp(LinearColor) (Variables|Default|GetSColor) (Variables|Default|GetEColor) (Variables|Default|GetAlpha)))
    (else
      (CallFunction|ChangeTempColor (Math|Color|Lerp(LinearColor) (Variables|Default|GetEColor) (Variables|Default|GetSColor) (Variables|Default|GetAlpha)))))
  (if (== 1.0 (Variables|Default|GetAlpha))
    (Variables|Default|SetAlpha 0.0)
    (Variables|Default|SetColorMove (not (Variables|Default|GetColorMove)))))

(event Custom|EndChangeColor
  (params (NewColor :type Linear%20Color%20Structure))
  (Utilities|Time|ClearandInvalidateTimerbyHandle (Variables|Default|GetLightHandle))
  (CallFunction|ChangeTempColor NewColor))

(event Custom|StartExtract
  (params (NewColor :type Linear%20Color%20Structure) (LerpColor :type Linear%20Color%20Structure))
  (Variables|Default|SetSColor NewColor)
  (Variables|Default|SetEColor LerpColor)
  (CallFunction|ChangeTempColor NewColor)
  (bind _returnvalue (Utilities|Time|SetTimerbyEvent (delegate Custom|CalcLerpColor) (Utilities|Time|GetWorldDeltaSeconds) true))
  (Variables|Default|SetLightHandle _returnvalue))

(event EventBeginPlay)

(event Collision|EventActorBeginOverlap
  (params (OtherActor :type Actor%20Object%20Reference)))

(event EventTick
  (params (DeltaSeconds :type Float%20%28single-precision%29)))

(fn ConstructionScript
  (bind _intensity (Variables|Light|GetIntensity))
  (bind _flickering (Variables|Light|GetFlickering))
  (bind _rotatingpart (Variables|Default|GetRotatingPart))
  ;[1 1 1] Change RotationParts Rotation
  (bind _output_get (Variables|Default|SetInitRotation_RotatingPart (Variables|/Script/Engine.SceneComponent|GetRelativeRotation _rotatingpart)))
  (Transformation|SetRelativeRotation _rotatingpart (Math|Rotator|MakeRotator (.Roll (Math|Rotator|BreakRotator _output_get)) (+ (.Pitch (Math|Rotator|BreakRotator _output_get)) (Variables|LightMesh|GetRotation)) (.Yaw (Math|Rotator|BreakRotator _output_get))) false false)
  ;[1 1 1] Hide One Mesh Part
  (Rendering|SetVisibility (Variables|Default|GetSM_StandingLight_A1_RotatingPart_N1) (Variables|LightMesh|GetOne/Two_Lights) false)
  ;[1 1 1] Light On/Off Toggle
  (if (Variables|Light|GetOn/Off)
    ;[1 1 1] Set RectLight Parameters
    (if (<= _intensity 0.0)
      ;[1 1 1] Change Material If Light Is Off
      (Rendering|Material|SetMaterial (Variables|Default|GetSM_StandingLight_A1_RotatingPart_N) 1 "/Game/Assets/Level/Prop/JUPITER_SciFi_Kit/Materials/MI_Light_Off.MI_Light_Off" :!label _label)
      (else
        ;[1 1 1] Set Light Material Parameters
        (bind _returnvalue (Rendering|Material|CreateDynamicMaterialInstance "/Game/Assets/Level/Prop/JUPITER_SciFi_Kit/Materials/MI_Light_Warm.MI_Light_Warm" "None" "None" :!class /Script/Engine.KismetMaterialLibrary))
        (Variables|Default|SetMI_TemporaryLight _returnvalue)
        (Rendering|Material|SetVectorParameterValue (Variables|Default|GetMI_TemporaryLight) "Light_Color" (Variables|Light|GetColor) :!class /Script/Engine.MaterialInstanceDynamic)
        (Rendering|Material|SetScalarParameterValue (Variables|Default|GetMI_TemporaryLight) "Light_Intencity" (/ _intensity 1.5e+03) :!class /Script/Engine.MaterialInstanceDynamic)
        (Rendering|Material|SetMaterial (Variables|Default|GetSM_StandingLight_A1_RotatingPart_N) 1 (Variables|Default|GetMI_TemporaryLight))
        ;[1 1 1] Flickering On/Off Toggle
        (if _flickering
          (Rendering|Material|SetScalarParameterValue (Variables|Default|GetMI_TemporaryLight) "Flickering" (Math|Conversions|ToFloat(Boolean) _flickering) :!class /Script/Engine.MaterialInstanceDynamic))))
    (else
      (goto _label))))