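; Extraction-point sci-fi sliding door that unlocks after a game-time delay, switching its decals from red to green.
; StartExtractWave triggers tagged enemies, extraction music and level-wide alarm lighting with timer-driven color pulsing.
; A looping CheckDoor timer polls open/close flags, counting down DoorOpenDelay before a Timeline slides the door.
; Trigger overlap notifies enemies of successful extraction and requests closing, after which EndLightChange applies cached light colors.
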(event OnComponentBeginOverlap(Door_Trigger)
  (params (OverlappedComponent :type Primitive%20Component%20Object%20Reference) (OtherActor :type Actor%20Object%20Reference) (OtherComp :type Primitive%20Component%20Object%20Reference) (OtherBodyIndex :type Integer) (bFromSweep :type Boolean) (SweepResult :type Hit%20Result%20Structure%20%28by%20ref%29))
  ;[1 1 1] Tigger overlapping. Set / reset door flags.
  (if (not (Variables|Default|GetWantDoorClose))
    (Variables|Default|SetWantDoorClose true)
    (Variables|Default|SetWantDoorOpen false)
    (bind _outactors (Actor|GetAllActorsOfClass "/Script/BODYCREDIT.CNox_EBase"))
    (for _array_element _outactors
      (Class|CNoxEBase|ExtractSucceed _array_element)
      (Variables|Default|SetbExtractSucceed true))))

(event OnComponentEndOverlap(Door_Trigger)
  (params (OverlappedComponent :type Primitive%20Component%20Object%20Reference) (OtherActor :type Actor%20Object%20Reference) (OtherComp :type Primitive%20Component%20Object%20Reference) (OtherBodyIndex :type Integer))
  ;[1 1 1] Tigger overlapping. Set / reset door flags.
  (Variables|Default|SetbExtractSucceed false)
  (Variables|Default|SetbStartExtract false))

(event Custom|ChangeTempColor
  (params (NewLightColor :type Linear%20Color%20Structure))
  ;[0.15 0.15 0.15 0.5] Light Color Change
  (Utilities|FlowControl|Sequence
    (:then_0
      (for _array_element (Variables|Default|GetPointLights)
        (Rendering|Components|Light|SetLightColor (Variables|/Script/Engine.PointLight|GetPointLightComponent _array_element) NewLightColor true)))
    (:then_1
      (for _array_element_2 (Variables|Default|GetRectLights)
        (Rendering|Components|Light|SetLightColor (Variables|/Script/Engine.RectLight|GetRectLightComponent _array_element_2) NewLightColor true)))
    (:then_2
      (for _array_element_3 (Variables|Default|GetSpotLights)
        (Rendering|Components|Light|SetLightColor (Variables|/Script/Engine.SpotLight|GetSpotLightComponent _array_element_3) NewLightColor true)))))

(event Custom|CalcLerpColor
  (Variables|Default|SetAlpha (Math|Float|Clamp(Float) (+ (Variables|Default|GetAlpha) (Utilities|Time|GetWorldDeltaSeconds))))
  (if (Variables|Default|GetColorMove)
    (CallFunction|ChangeTempColor (Math|Color|Lerp(LinearColor) (Variables|Default|GetSLightLerpColor) (Variables|Default|GetELightLerpColor) (Variables|Default|GetAlpha)))
    (else
      (CallFunction|ChangeTempColor (Math|Color|Lerp(LinearColor) (Variables|Default|GetELightLerpColor) (Variables|Default|GetSLightLerpColor) (Variables|Default|GetAlpha)))))
  (if (== 1.0 (Variables|Default|GetAlpha))
    (Variables|Default|SetAlpha 0.0)
    (Variables|Default|SetColorMove (not (Variables|Default|GetColorMove)))))

(event Custom|SetLightArray
  ;[0.15 0.15 0.15 0.5] Make Light Color Array
  (Utilities|FlowControl|Sequence
    (:then_0
      (bind _outactors (Actor|GetAllActorsOfClass "/Script/Engine.PointLight"))
      (bind _output_get (Variables|Default|SetPointLights _outactors))
      (for _array_element _output_get
        (Utilities|Array|Add (Variables|Default|GetOrgColor) (Rendering|Components|Light|GetLightColor (Variables|/Script/Engine.PointLight|GetPointLightComponent _array_element)))))
    (:then_1
      (bind _outactors_2 (Actor|GetAllActorsOfClass "/Script/Engine.RectLight"))
      (bind _output_get_2 (Variables|Default|SetRectLights _outactors_2))
      (for _array_element_2 _output_get_2
        (Utilities|Array|Add (Variables|Default|GetOrgColor) (Rendering|Components|Light|GetLightColor (Variables|/Script/Engine.RectLight|GetRectLightComponent _array_element_2)))))
    (:then_2
      (bind _outactors_3 (Actor|GetAllActorsOfClass "/Script/Engine.SpotLight"))
      (bind _output_get_3 (Variables|Default|SetSpotLights _outactors_3))
      (for _array_element_3 _output_get_3
        (Utilities|Array|Add (Variables|Default|GetOrgColor) (Rendering|Components|Light|GetLightColor (Variables|/Script/Engine.SpotLight|GetSpotLightComponent _array_element_3)))))
    (:then_3
      (bind _outactors_4 (Actor|GetAllActorsOfClass "/Game/JUPITER_SciFi_Kit/Blueprints/BP_StandingLight_A1_N.BP_StandingLight_A1_N_C"))
      (bind _output_get_4 (Variables|Default|SetStands1 _outactors_4))
      (for _array_element_4 _output_get_4
        (Utilities|Array|Add (Variables|Default|GetOrgColor) (Variables|/Game/JUPITER_SciFi_Kit/Blueprints/BP_StandingLight_A1_N.BP_StandingLight_A1_N_C|GetColor _array_element_4))))
    (:then_4
      (bind _outactors_5 (Actor|GetAllActorsOfClass "/Game/JUPITER_SciFi_Kit/Blueprints/BP_StandingLight_A2_N.BP_StandingLight_A2_N_C"))
      (bind _output_get_5 (Variables|Default|SetStands2 _outactors_5))
      (for _array_element_5 _output_get_5
        (Utilities|Array|Add (Variables|Default|GetOrgColor) (Variables|/Game/JUPITER_SciFi_Kit/Blueprints/BP_StandingLight_A2_N.BP_StandingLight_A2_N_C|GetColor _array_element_5))))
    (:then_5
      (bind _outactors_6 (Actor|GetAllActorsOfClass "/Game/JUPITER_SciFi_Kit/Blueprints/BP_Light_A1_5X1_N.BP_Light_A1_5X1_N_C"))
      (bind _output_get_6 (Variables|Default|SetLights5 _outactors_6))
      (for _array_element_6 _output_get_6
        (Utilities|Array|Add (Variables|Default|GetOrgColor) (Variables|/Game/JUPITER_SciFi_Kit/Blueprints/BP_Light_A1_5X1_N.BP_Light_A1_5X1_N_C|GetColor _array_element_6))))
    (:then_6
      (bind _outactors_7 (Actor|GetAllActorsOfClass "/Game/JUPITER_SciFi_Kit/Blueprints/BP_Light_A1_3X1_N.BP_Light_A1_3X1_N_C"))
      (bind _output_get_7 (Variables|Default|SetLights3 _outactors_7))
      (for _array_element_7 _output_get_7
        (Utilities|Array|Add (Variables|Default|GetOrgColor) (Variables|/Game/JUPITER_SciFi_Kit/Blueprints/BP_Light_A1_3X1_N.BP_Light_A1_3X1_N_C|GetColor _array_element_7))))
    (:then_7
      (bind _directionallightobj (Variables|Default|GetDirectionalLightObj)
        (:then
          (Utilities|Array|Add (Variables|Default|GetOrgColor) (Rendering|Components|Light|GetLightColor (Variables|/Script/Engine.Light|GetLightComponent _directionallightobj)))
          (bind _fogobj (Variables|Default|GetFogObj)
            (:then
              (Utilities|Array|Add (Variables|Default|GetOrgColor) (Variables|/Script/Engine.ExponentialHeightFogComponent|GetFogInscatteringLuminance (Variables|/Script/Engine.ExponentialHeightFog|GetComponent _fogobj))))
            (:else)))
        (:else)))))

(event Custom|ResetEventPlayerDie
  (CallFunction|CloseDoor)
  ;[1 1 1] Main door state flag:
  ; True = door Open
  ; False = door Closed
  (Variables|Default|SetIsDoorOpen false)
  ;[1 1 1] Door Flags: WantClose - if player leave trigger volume.
  ; WantOpen - if player inside of trigger doors
  (Variables|Default|SetWantDoorOpen false)
  (Variables|Default|SetWantDoorClose false)
  (Variables|Default|SetIsDoorInProgress false))

(event Custom|CheckDoor
  ;[0.3708 0.3656 1] Main logic. Check door state. Checking every 0.5 seconds.
  (bind _gm (Variables|Default|GetGM)
    (:then
      (bind _returnvalue (Class|CMainGM|GetGamePlayTime _gm))
      (if (> _returnvalue (Variables|Default|GetExtractDelay))
        (Utilities|FlowControl|Sequence
          (:then_0
            (if (not (Variables|Default|GetIsDoorInProgress))
              (if (Variables|Default|GetWantDoorOpen)
                ;;[1 1 1] Ensure that door closed then process to Open
                (if (not (Variables|Default|GetIsDoorOpen))
                  (CallFunction|OpenDoor))
                (elif (Variables|Default|GetWantDoorClose)
                  ;;[1 1 1] Ensure that door is opened then process to Close
                  (if (Variables|Default|GetIsDoorOpen)
                    (Variables|Default|SetWantDoorClose false)
                    (CallFunction|CloseDoor))))))
          (:then_1
            (if (not (Variables|Default|GetIsChangeColor))
              (CallFunction|DecalColorChange)
              (Variables|Default|SetIsChangeColor true))))))
    (:else)))

(event Custom|StartExtract_ChangeColor
  (params (NewColor :type Linear%20Color%20Structure) (LerpColor :type Linear%20Color%20Structure))
  (CallFunction|ChangeTempColor NewColor)
  (bind _returnvalue (Utilities|Time|SetTimerbyEvent (delegate Custom|CalcLerpColor) (Utilities|Time|GetWorldDeltaSeconds) true))
  (Variables|Default|SetLightHandle _returnvalue))

(event Custom|StartLightChange
  ;[0.15 0.15 0.15 0.5] Start Light Change
  (Utilities|FlowControl|Sequence
    (:then_0
      (CallFunction|ChangeTempColor (Variables|Default|GetSLightLerpColor)))
    (:then_1
      (for _array_element (Variables|Default|GetStands1)
        (Default|StartExtract _array_element (Variables|Default|GetSLampLerpColor) (Variables|Default|GetELampLerpColor))))
    (:then_2
      (for _array_element_2 (Variables|Default|GetStands2)
        (Default|StartExtract _array_element_2 (Variables|Default|GetSLampLerpColor) (Variables|Default|GetELampLerpColor))))
    (:then_3
      (for _array_element_3 (Variables|Default|GetLights5)
        (Default|StartExtract _array_element_3 (Variables|Default|GetSLampLerpColor) (Variables|Default|GetELampLerpColor))))
    (:then_4
      (for _array_element_4 (Variables|Default|GetLights3)
        (Default|StartExtract _array_element_4 (Variables|Default|GetSLampLerpColor) (Variables|Default|GetELampLerpColor))))
    (:then_5
      (CallFunction|StartExtractChangeColor)
      (Utilities|FlowControl|Sequence
        (:then_0
          (bind _directionallightobj (Variables|Default|GetDirectionalLightObj)
            (:then
              (Rendering|Components|Light|SetLightColor (Variables|/Script/Engine.Light|GetLightComponent _directionallightobj) "(R=1.000000,G=0.505882,B=0.564706,A=1.000000)" true))
            (:else)))
        (:then_1
          (bind _fogobj (Variables|Default|GetFogObj)
            (:then
              (Class|ExponentialHeightFogComponent|SetFogInscatteringColor (Variables|/Script/Engine.ExponentialHeightFog|GetComponent _fogobj) "(R=0.721569,G=0.380392,B=0.309804,A=1.000000)"))
            (:else)))))))

(event Custom|CloseDoor
  (bind _initdoorlocation (Variables|Default|GetInitDoorLocation))
  ;[1 1 1] Open/Close animtation. Just pick valuer from time line and set Z location for door halfs
  (Variables|Default|SetIsDoorInProgress true)
  ;;[1 0.03484 0.1445] Change door state
  (Variables|Default|SetIsDoorOpen false)
  (bind _newtrack_0 (Timeline|Timeline_0 ReverseFromEnd)
    (:Update
      (Transformation|SetRelativeLocation (Variables|Default|GetDoor) (Math|Vector|MakeVector (.x _initdoorlocation) (+ (* _newtrack_0 (Variables|Default|GetDoorOpenLimit)) (.y _initdoorlocation)) (.z _initdoorlocation)) false false))
    (:Finished
      (Variables|Default|SetIsDoorInProgress false)
      (if (not (Variables|Default|GetIsDoorOpen))
        (CallFunction|EndLightChange)
        (Variables|Default|SetCurResetColorIdx 0)))))

(event Custom|OpenDoor
  (bind _initdoorlocation (Variables|Default|GetInitDoorLocation))
  ;[1 1 1] Open/Close animtation. Just pick valuer from time line and set Z location for door halfs
  (bind _output_get (Variables|Default|SetDoorOpenDelay (- (Variables|Default|GetDoorOpenDelay) (Class|KismetSystemLibrary|GetTimerElapsedTimeHandle (Variables|Default|GetCheckDoorTimeHandle)))))
  (if (<= _output_get 0.0)
    (Variables|Default|SetWantDoorOpen false)
    (Variables|Default|SetIsDoorInProgress true)
    ;;[1 0.03484 0.1445] Change door state
    (Variables|Default|SetIsDoorOpen true)
    (bind _newtrack_0 (Timeline|Timeline_0 PlayFromStart)
      (:Update
        (Transformation|SetRelativeLocation (Variables|Default|GetDoor) (Math|Vector|MakeVector (.x _initdoorlocation) (+ (* _newtrack_0 (Variables|Default|GetDoorOpenLimit)) (.y _initdoorlocation)) (.z _initdoorlocation)) false false))
      (:Finished
        (Variables|Default|SetIsDoorInProgress false)
        (if (not (Variables|Default|GetIsDoorOpen))
          (CallFunction|EndLightChange)
          (Variables|Default|SetCurResetColorIdx 0))))))

(event Custom|StartExtractWave
  (params (Player :type BP%20C%20Nox%20Runner%20Object%20Reference))
  (if (and (not (Variables|Default|GetbExtractSucceed)) (not (Variables|Default|GetbStartExtract)))
    (bind _gm (Variables|Default|GetGM)
      (:then
        (bind _returnvalue (Class|CMainGM|GetGamePlayTime _gm))
        (if (> _returnvalue (Variables|Default|GetExtractDelay))
          (bind _outactors (Actor|GetAllActorsOfClasswithTag "/Script/BODYCREDIT.CNox_EBase" "Enemy"))
          (for _array_element _outactors
            (Class|CNoxEBase|ExtractCallFunction _array_element Player))
          (CallFunction|StartLightChange)
          (Variables|Default|SetWantDoorOpen true)
          (Variables|Default|SetWantDoorClose false)
          (bind _asbp_net_game_instance (Utilities|Casting|CastToBP_NetGameInstance (Game|GetGameInstance)))
          (Class|NetGameInstance|PlayBGM _asbp_net_game_instance 2)
          (Variables|Default|SetbStartExtract true)))
      (:else))))

(event Custom|DecalColorChange
  (bind _mi_decal (Variables|Default|GetMI_Decal))
  (bind _sm_door_a1_3x2_n (Variables|Default|GetSM_Door_A1_3X2_N))
  (bind _sm_door_a1_3x2_n1 (Variables|Default|GetSM_Door_A1_3X2_N1))
  (Rendering|Material|SetVectorParameterValue _mi_decal "Emissive_Color" (Variables|Default|GetGreenColor) :!class /Script/Engine.MaterialInstanceDynamic)
  (Rendering|Material|SetMaterial _sm_door_a1_3x2_n 2 _mi_decal)
  (Rendering|Material|SetMaterial _sm_door_a1_3x2_n 3 _mi_decal)
  (Rendering|Material|SetMaterial _sm_door_a1_3x2_n1 2 _mi_decal)
  (Rendering|Material|SetMaterial _sm_door_a1_3x2_n1 3 _mi_decal))

(event Custom|EndLightChange
  ;[0.15 0.15 0.15 0.5] Return Origin Color
  (Utilities|Time|ClearandInvalidateTimerbyHandle (Variables|Default|GetLightHandle))
  (for _array_element (Variables|Default|GetOrgColor)
    (switch int (Variables|Default|GetCurResetColorIdx)
      (:0
        (for _array_element_2 (Variables|Default|GetPointLights)
          (Rendering|Components|Light|SetLightColor (Variables|/Script/Engine.PointLight|GetPointLightComponent _array_element_2) _array_element true))
        (Math|Integer|IncrementInt (Variables|Default|GetCurResetColorIdx) :!label _label))
      (:1
        (for _array_element_3 (Variables|Default|GetRectLights)
          (Rendering|Components|Light|SetLightColor (Variables|/Script/Engine.RectLight|GetRectLightComponent _array_element_3) _array_element true))
        (goto _label))
      (:2
        (for _array_element_4 (Variables|Default|GetSpotLights)
          (Rendering|Components|Light|SetLightColor (Variables|/Script/Engine.SpotLight|GetSpotLightComponent _array_element_4) _array_element true))
        (goto _label))
      (:3
        (for _array_element_5 (Variables|Default|GetStands1)
          (Default|EndChangeColor _array_element_5 _array_element))
        (goto _label))
      (:4
        (for _array_element_6 (Variables|Default|GetStands2)
          (Default|EndChangeColor _array_element_6 _array_element))
        (goto _label))
      (:5
        (for _array_element_7 (Variables|Default|GetLights5)
          (Default|EndChangeColor _array_element_7 _array_element))
        (goto _label))
      (:6
        (for _array_element_8 (Variables|Default|GetLights3)
          (Default|EndChangeColor _array_element_8 _array_element))
        (goto _label))
      (:7
        (bind _directionallightobj (Variables|Default|GetDirectionalLightObj)
          (:then
            (Rendering|Components|Light|SetLightColor (Variables|/Script/Engine.Light|GetLightComponent _directionallightobj) _array_element true)
            (goto _label))
          (:else
            (goto _label))))
      (:8
        (bind _fogobj (Variables|Default|GetFogObj)
          (:then
            (Class|ExponentialHeightFogComponent|SetFogInscatteringColor (Variables|/Script/Engine.ExponentialHeightFog|GetComponent _fogobj) _array_element))
          (:else))))))

(event EventBeginPlay
  ;[1 1 1] Main door state flag:
  ; True = door Open
  ; False = door Closed
  (Variables|Default|SetIsDoorOpen false)
  ;[1 1 1] Door Flags: WantClose - if player leave trigger volume.
  ; WantOpen - if player inside of trigger doors
  (Variables|Default|SetWantDoorOpen false)
  (Variables|Default|SetWantDoorClose false)
  (Variables|Default|SetIsDoorInProgress false)
  ;[1 1 1] Store initial door locations
  (Variables|Default|SetInitDoorLocation (Variables|/Script/Engine.SceneComponent|GetRelativeLocation (Variables|Default|GetDoor)))
  ;[0.3708 0.3656 1] Timer! Each 0,5 sec we will check a door flags by executing CheckDoors event
  (bind _returnvalue (Utilities|Time|SetTimerbyFunctionName 0 "CheckDoor" 0.1 true))
  (bind _output_get (Variables|Default|SetCheckDoorTimeHandle _returnvalue))
  (Utilities|Time|UnpauseTimerbyHandle _output_get)
  (bind _asbp_cmain_gm (Utilities|Casting|CastToBP_CMainGM (Game|GetGameMode)))
  (Variables|Default|SetGM _asbp_cmain_gm)
  (CallFunction|SetLightArray))

(fn ConstructionScript
  (bind _sm_door_a1_3x2_n (Variables|Default|GetSM_Door_A1_3X2_N))
  (bind _sm_door_a1_3x2_n1 (Variables|Default|GetSM_Door_A1_3X2_N1))
  (bind _returnvalue (Rendering|Material|CreateDynamicMaterialInstance "/Game/JUPITER_SciFi_Kit/Materials/MI_DecalsSet.MI_DecalsSet" "None" "None" :!class /Script/Engine.KismetMaterialLibrary))
  (Variables|Default|SetMI_Decal _returnvalue)
  (Rendering|Material|SetVectorParameterValue (Variables|Default|GetMI_Decal) "Emissive_Color" (Variables|Default|GetRedColor) :!class /Script/Engine.MaterialInstanceDynamic)
  (Rendering|Material|SetMaterial _sm_door_a1_3x2_n 2 (Variables|Default|GetMI_Decal))
  (Rendering|Material|SetMaterial _sm_door_a1_3x2_n 3 (Variables|Default|GetMI_Decal))
  (Rendering|Material|SetMaterial _sm_door_a1_3x2_n1 2 (Variables|Default|GetMI_Decal))
  (Rendering|Material|SetMaterial _sm_door_a1_3x2_n1 3 (Variables|Default|GetMI_Decal)))